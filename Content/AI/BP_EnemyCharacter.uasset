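; Enemy AI character with a world-space health bar that drops a fuel cell pickup when killed.
; BeginPlay seeds the WBP_EnemyBoss_HP widget, and Tick turns it toward the player camera.
; ModifyHealth subtracts damage, updates the bar, and either flags death or rotates the enemy toward the player.
; Tick polls IsDead to detach the controller, then after a delay spawns particles and BP_Item_FuelCell2 before destroying the actor.
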(event `self.ReceiveBeginPlay`
  (`self.InitializeHealthbar`))

(event `self.ReceiveTick`
  (params (DeltaSeconds :type "Float (single-precision)"))
  (bind _particlesystemtarget (`self.ParticleSystemTarget`))
  (`self.RotateHealthbarTowardsPlayer`)
  (if (`self.isDead`)
    (`self.DetachFromControllerPendingDestroy`) ; Stop all behavior tree movement
    (`KismetSystemLibrary.Delay` 3.0)
    (`GameplayStatics.SpawnEmitterAtLocation` "/Game/ParticleSystems/PS_BrightCubes.PS_BrightCubes" (`SceneComponent.K2_GetComponentLocation` _particlesystemtarget))
    (`|SpawnActorFromClass` "/Game/Blueprints/InventorySystem/Item/BP_Item_FuelCell2.BP_Item_FuelCell2_C" (`KismetMathLibrary.MakeTransform` (+ (`SceneComponent.K2_GetComponentLocation` _particlesystemtarget) (0.0 0.0 -45.0))) "Undefined" "OverrideRootScale" null null)
    (`self.K2_DestroyActor`)))

(fn `InitializeHealthbar`
  (bind _health (`self.health`))
  (bind _aswbp_enemy_boss_hp (cast `/Game/Blueprints/UI/WBP_EnemyBoss_HP` (`WidgetComponent.GetUserWidgetObject` (`self.Healthbar`))))
  (bind _output_get (set `self.WidgetHealthbar` _aswbp_enemy_boss_hp))
  (set `/Game/Blueprints/UI/WBP_EnemyBoss_HP.health` _health _output_get)
  (set `/Game/Blueprints/UI/WBP_EnemyBoss_HP.maxHealth` (`self.maxHealth`) _output_get)
  (`/Game/Blueprints/UI/WBP_EnemyBoss_HP.UpdateHealth` _output_get _health))

(fn `ModifyHealth`
  (params (healthToSubtract :type "Float (double-precision)"))
  (bind _returnvalue (- (`self.health`) healthToSubtract))
  (if (<= _returnvalue 0.0)
    (set `self.isDead` true)
    (bind _output_get (set `self.health` 0.0))
    (`/Game/Blueprints/UI/WBP_EnemyBoss_HP.UpdateHealth` (`self.WidgetHealthbar`) _output_get)
    (else
      (bind _output_get_2 (set `self.health` _returnvalue))
      (`/Game/Blueprints/UI/WBP_EnemyBoss_HP.UpdateHealth` (`self.WidgetHealthbar`) _output_get_2)
      (`self.K2_SetActorRotation` (`KismetMathLibrary.RInterpTo` (`self.K2_GetActorRotation`) (`KismetMathLibrary.FindLookAtRotation` (`self.K2_GetActorLocation`) (`self.K2_GetActorLocation` (`GameplayStatics.GetPlayerCharacter` 0))) 25.0 5.0)) ; Force AI to face the player
    )))

(fn `RotateHealthbarTowardsPlayer`
  (bind (_returnvalue_roll _returnvalue_pitch _returnvalue_yaw) (`KismetMathLibrary.BreakRotator` (`KismetMathLibrary.FindLookAtRotation` (`SceneComponent.K2_GetComponentLocation` (`PlayerCameraManager.TransformComponent` (`GameplayStatics.GetPlayerCameraManager` 0))) (`SceneComponent.K2_GetComponentLocation` (`self.Healthbar`)))))
  (`SceneComponent.K2_SetWorldRotation` (`self.Healthbar`) (`KismetMathLibrary.MakeRotator` _returnvalue_roll (* _returnvalue_pitch -1.0) (+ _returnvalue_yaw 180.0)) false false))

(fn `UserConstructionScript`)