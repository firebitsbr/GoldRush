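; Cabin actor that lifts and fades out its roof while the player character is inside its trigger box.
; Overlap begin and end play the RemoveRoof and PlaceRoof timelines, which raise or lower the roof incrementally from its current location, clamping world Z between zero and RemoveHeight.
; The same timelines drive opacity on two dynamic roof material instances created in the construction script.
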(event `self.TriggerBox.OnComponentBeginOverlap`
  (params (OverlappedComponent :type "PrimitiveComponent Object Reference") (OtherActor :type "Actor Object Reference") (OtherComp :type "PrimitiveComponent Object Reference") (OtherBodyIndex :type Integer) (bFromSweep :type Boolean) (SweepResult :type "HitResult Structure (by ref)"))
  (bind (_returnvalue_x _returnvalue_y _returnvalue_z) (`KismetMathLibrary.BreakVector` (`SceneComponent.K2_GetComponentLocation` (`self.Roof`))))
  (if (== OtherActor (`GameplayStatics.GetPlayerCharacter` 0))
    (bind (_direction _floatlerp) (`Timeline|RemoveRoof` :!via `PlayFromStart`)
      (:`Update`
        (bind (_returnvalue_x_2 _returnvalue_y_2 _returnvalue_z_2) (`KismetMathLibrary.BreakVector` (`KismetMathLibrary.VLerp` (`KismetMathLibrary.MakeVector` _returnvalue_x _returnvalue_y _returnvalue_z) (`KismetMathLibrary.MakeVector` _returnvalue_x _returnvalue_y (+ _returnvalue_z (`self.RemoveSpeed`))) _floatlerp)))
        (`SceneComponent.K2_SetWorldLocation` (`self.Roof`) (`KismetMathLibrary.MakeVector` _returnvalue_x_2 _returnvalue_y_2 (`KismetMathLibrary.FClamp` _returnvalue_z_2 0.0 (`self.RemoveHeight`))) false false)
        (bind _returnvalue (`KismetMathLibrary.Lerp` 1.0 0.0 (* _floatlerp 1.33)))
        (`MaterialInstanceDynamic.SetScalarParameterValue` (`self.ShedRoofMaterialInst`) "Opacity" _returnvalue)
        (`MaterialInstanceDynamic.SetScalarParameterValue` (`self.RoofMaterialInst`) "Opacity" _returnvalue)))))

(event `self.TriggerBox.OnComponentEndOverlap`
  (params (OverlappedComponent :type "PrimitiveComponent Object Reference") (OtherActor :type "Actor Object Reference") (OtherComp :type "PrimitiveComponent Object Reference") (OtherBodyIndex :type Integer))
  (bind (_returnvalue_x _returnvalue_y _returnvalue_z) (`KismetMathLibrary.BreakVector` (`SceneComponent.K2_GetComponentLocation` (`self.Roof`))))
  (if (== OtherActor (`GameplayStatics.GetPlayerCharacter` 0))
    (bind (_direction _floatscale) (`Timeline|PlaceRoof` :!via `PlayFromStart`)
      (:`Update`
        (bind (_returnvalue_x_2 _returnvalue_y_2 _returnvalue_z_2) (`KismetMathLibrary.BreakVector` (`KismetMathLibrary.VLerp` (`KismetMathLibrary.MakeVector` _returnvalue_x _returnvalue_y _returnvalue_z) (`KismetMathLibrary.MakeVector` _returnvalue_x _returnvalue_y (- _returnvalue_z (`self.RemoveSpeed`))) _floatscale)))
        (`SceneComponent.K2_SetWorldLocation` (`self.Roof`) (`KismetMathLibrary.MakeVector` _returnvalue_x_2 _returnvalue_y_2 (`KismetMathLibrary.FClamp` _returnvalue_z_2 0.0 (`self.RemoveHeight`))) false false)
        (bind _returnvalue (`KismetMathLibrary.Lerp` 0.0 1.0 _floatscale))
        (`MaterialInstanceDynamic.SetScalarParameterValue` (`self.ShedRoofMaterialInst`) "Opacity" _returnvalue)
        (`MaterialInstanceDynamic.SetScalarParameterValue` (`self.RoofMaterialInst`) "Opacity" _returnvalue)))))

(fn `UserConstructionScript`
  (bind _returnvalue (`PrimitiveComponent.CreateDynamicMaterialInstance` (`self.Roof`) 0 "/Game/Materials/Cabin/M_Cabin_Shed_Roof_Inst.M_Cabin_Shed_Roof_Inst" "None"))
  (set `self.ShedRoofMaterialInst` _returnvalue)
  (bind _returnvalue_2 (`PrimitiveComponent.CreateDynamicMaterialInstance` (`self.Roof`) 1 "/Game/Materials/Cabin/M_Cabin_Roof_Inst.M_Cabin_Roof_Inst" "None"))
  (set `self.RoofMaterialInst` _returnvalue_2))