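; Base Blueprint for world items in the inventory system, showing a spinning, bobbing mesh that opens an interaction window on interact.
; Interact creates a single WBP_InteractWindow from ItemStructure's name, description and thumbnail on the player controller's HUD canvas.
; Leaving the collision sphere removes that window.
; Tick turns the ClickToInteract widget toward the camera and offsets the mesh, using a Delay to flip the vertical direction.
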(event `/Game/Blueprints/InventorySystem/BPI_Interact.interact`
  (params (Interactor :type "Actor Object Reference"))
  ;[1 1 1] Check if a menu is already open
  (if (not (`KismetSystemLibrary.IsValid` (`self.InteractWindow`)))
    (`self.ShowInteractWindow` Interactor)))

(event `self.Sphere Collision.OnComponentEndOverlap`
  (params (OverlappedComponent :type "PrimitiveComponent Object Reference") (OtherActor :type "Actor Object Reference") (OtherComp :type "PrimitiveComponent Object Reference") (OtherBodyIndex :type Integer))
  ;[1 1 1] Remove the widget when player exits the collision sphere
  (`self.CloseUI`))

(event `self.ReceiveTick`
  (params (DeltaSeconds :type "Float (single-precision)"))
  (bind _staticmesh (`self.StaticMesh`))
  (`self.RotateWidgetToFaceCamera`)
  (`SceneComponent.K2_SetWorldLocationAndRotation` (`self.StaticMesh`) (`KismetMathLibrary.MakeVector` (.x (`SceneComponent.K2_GetComponentLocation` _staticmesh)) (.y (`SceneComponent.K2_GetComponentLocation` _staticmesh)) (+ (.z (`SceneComponent.K2_GetComponentLocation` _staticmesh)) (`self.translationOffset`))) (`KismetMathLibrary.MakeRotator` (.roll (`SceneComponent.K2_GetComponentRotation` _staticmesh)) (.pitch (`SceneComponent.K2_GetComponentRotation` _staticmesh)) (+ (.yaw (`SceneComponent.K2_GetComponentRotation` _staticmesh)) (`self.rotationOffset`))) false false)
  ;[1 1 1] Raises the item up and down
  (`KismetSystemLibrary.Delay` 0.7)
  (if (== (`self.translationOffset`) 1.0)
    (set `self.translationOffset` -1.0)
    (else
      (set `self.translationOffset` 1.0)))
  ;[1 1 1] Continuously rotate the item 360 degrees
  (if (== (`self.rotationOffset`) 360.0)
    (set `self.rotationOffset` 0.0)))

(fn `CloseUI`
  (bind _interactwindow (`self.InteractWindow`))
  ;[1 1 1] Checks if an instance of InspectWindow already exists or not
  (if (`KismetSystemLibrary.IsValid` _interactwindow)
    (`Widget.RemoveFromParent` _interactwindow)
    (set `self.InteractWindow` null)))

(fn `RotateWidgetToFaceCamera`
  (bind (_returnvalue_roll _returnvalue_pitch _returnvalue_yaw) (`KismetMathLibrary.BreakRotator` (`KismetMathLibrary.FindLookAtRotation` (`SceneComponent.K2_GetComponentLocation` (`PlayerCameraManager.TransformComponent` (`GameplayStatics.GetPlayerCameraManager` 0))) (`SceneComponent.K2_GetComponentLocation` (`self.ClickToInteract`)))))
  (`SceneComponent.K2_SetWorldRotation` (`self.ClickToInteract`) (`KismetMathLibrary.MakeRotator` _returnvalue_roll (* _returnvalue_pitch -1.0) (+ _returnvalue_yaw 180.0)) false false))

(fn `ShowInteractWindow`
  (params (Interactor :type "Actor Object Reference"))
  (bind (_itemstructure_name _itemstructure_thumbnail _itemstructure_description) (break `/Game/Blueprints/InventorySystem/ItemStructure` (`self.ItemStructure`)))
  (bind _returnvalue (`|CreateWidget` "/Game/Blueprints/UI/WBP_InteractWindow.WBP_InteractWindow_C" null self _itemstructure_name _itemstructure_description _itemstructure_thumbnail Interactor))
  (set `self.InteractWindow` _returnvalue)
  (bind _asbp_player_controller (cast `/Game/Blueprints/Character/Player/BP_PlayerController` (`GameplayStatics.GetPlayerController` 0)))
  (bind _returnvalue_2 (`CanvasPanel.AddChildToCanvas` (`/Game/Blueprints/UI/WBP_HUD.HudCanvas` (`/Game/Blueprints/Character/Player/BP_PlayerController.HudWidget` _asbp_player_controller)) (`self.InteractWindow`)))
  (`CanvasPanelSlot.SetAutoSize` _returnvalue_2 true)
  (`CanvasPanelSlot.SetAlignment` _returnvalue_2 (0.5 0.5))
  (`CanvasPanelSlot.SetAnchors` _returnvalue_2 (make `Anchors` (0.5 0.5) (0.5 0.5)))
  (`CanvasPanelSlot.SetPosition` _returnvalue_2 (0.0 180.0)))

(fn `UserConstructionScript`)