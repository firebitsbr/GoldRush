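; Inventory component that holds items in a slot array sized on BeginPlay and shows them in a window on the TopDownController's HUD canvas.
; Adding writes content into the first slot matching an empty slot structure, without merging stacks, and always reports success.
; Toggling creates or removes the center-anchored window.
; Removing deletes the array element, shrinking the array, and rebuilds the window if open, while adding does not refresh it.
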(event `self.ReceiveBeginPlay`
  (`self.PrepareInventory`))

(event `RefreshInventory`
  (`Widget.RemoveFromParent` (`self.InventoryWindow`)) ; Remove existing UI
  (bind _returnvalue (`|CreateWidget` "/Game/Blueprints/UI/WBP_InventoryWindow.WBP_InventoryWindow_C" null self))
  (set `self.InventoryWindow` _returnvalue)
  (bind _astop_down_controller (cast `/Game/Blueprints/Character/Player/TopDownController` (`GameplayStatics.GetPlayerController` 0)))
  (bind _returnvalue_2 (`CanvasPanel.AddChildToCanvas` (`/Game/Blueprints/UI/WBP_HUD.HudCanvas` (`/Game/Blueprints/Character/Player/TopDownController.HudWidget` _astop_down_controller)) (`self.InventoryWindow`)))
  (`CanvasPanelSlot.SetAutoSize` _returnvalue_2 true)
  (`CanvasPanelSlot.SetAlignment` _returnvalue_2 (0.5 0.5))
  (`CanvasPanelSlot.SetAnchors` _returnvalue_2 (make `Anchors` (0.5 0.5) (0.5 0.5)))
  (`CanvasPanelSlot.SetPosition` _returnvalue_2 (`self.position`)))

(fn `AddToInventory`
  (params (ContentToAdd :type "/Game/Blueprints/InventorySystem/SlotStructure Structure"))
  (returns (Success :type Boolean))
  (`self.CreateStack` ContentToAdd)
  (return true))

(fn `CreateStack`
  (params (ContentToAdd :type "/Game/Blueprints/InventorySystem/SlotStructure Structure"))
  (bind _inventory (`self.inventory`))
  (`KismetArrayLibrary.Array_Set` _inventory (`KismetArrayLibrary.Array_Find` _inventory (make `/Game/Blueprints/InventorySystem/SlotStructure` (struct))) ContentToAdd))

(fn `PrepareInventory`
  (`KismetArrayLibrary.Array_Resize` (`self.inventory`) (`self.numberOfSlots`)))

(fn `RemoveFromInventory`
  (params (Item_Index :type Integer))
  (`KismetArrayLibrary.Array_Remove` (`self.inventory`) Item_Index)
  (`self.InventoryWindow`
    (:`then`
      (`self.RefreshInventory`))
    (:`else`)))

(fn `ToggleInventory`
  ;[1 1 1] Checks to see if the inventory window already exists or not
  (`self.InventoryWindow`
    (:`then`
      (`Widget.RemoveFromParent` (`self.InventoryWindow`))
      (set `self.InventoryWindow` null))
    (:`else`
      (bind _returnvalue (`|CreateWidget` "/Game/Blueprints/UI/WBP_InventoryWindow.WBP_InventoryWindow_C" null self))
      (set `self.InventoryWindow` _returnvalue)
      (bind _astop_down_controller (cast `/Game/Blueprints/Character/Player/TopDownController` (`GameplayStatics.GetPlayerController` 0)))
      (bind _returnvalue_2 (`CanvasPanel.AddChildToCanvas` (`/Game/Blueprints/UI/WBP_HUD.HudCanvas` (`/Game/Blueprints/Character/Player/TopDownController.HudWidget` _astop_down_controller)) (`self.InventoryWindow`)))
      (`CanvasPanelSlot.SetAutoSize` _returnvalue_2 true)
      (`CanvasPanelSlot.SetAlignment` _returnvalue_2 (0.5 0.5))
      (`CanvasPanelSlot.SetAnchors` _returnvalue_2 (make `Anchors` (0.5 0.5) (0.5 0.5)))
      (`CanvasPanelSlot.SetPosition` _returnvalue_2 (`self.position`)))))